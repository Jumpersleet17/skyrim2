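; Animated tile-toolkit unit Blueprint that adds Animation Blueprint-driven animation and a health bar to its parent unit.
; Movement updates, via a multicast event, and ability actions are forwarded as messages to the mesh's AnimInstance.
; A dynamic material's PercentFill shows health as CurrentHealth over MaxHealth.
; Hurt handling refreshes the bar, then at zero health ends the action, queues Death and stops movement; death hides the bar.
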(event Custom|MulticastMoveAnimation
  (Class|BPIAnimateUnit|AnimateMovement(Message) (Variables|Default|GetAbpRef) (Variables|Default|GetCurrentSpeed)))

(event EventAnimateDeath
  (params (Action :type F%20Action%20Structure))
  (|CallParentFunction Action)
  (Rendering|SetVisibility (Variables|Default|GetHealthBar) false false))

(event EventAnimateUnit
  (params (Action :type F%20Action%20Structure%20%28by%20ref%29))
  (Class|BPIAnimateUnit|AnimateAbility(Message) (Variables|Default|GetAbpRef) Action))

(event EventTimelineMoveUpdateFunc
  (|CallParentFunction)
  (CallFunction|MulticastMoveAnimation))

(event EventBeginPlay
  (|CallParentFunction)
  (Variables|Default|SetAbpRef (Components|SkeletalMesh|GetAnimInstance (Variables|Default|GetMesh))))

(event EventAnimateHurt
  (params (Action :type F%20Action%20Structure) (Damage :type Float%20%28single-precision%29))
  (bind _bempty (CallFunction|ModifyHealthBar (* Damage -1.0)))
  (if _bempty
    (Class|BPIAction|EndAction(Message) (Game|GetGameState))
    (Utilities|SimpleQueue "NewEnumerator1" self "Death" false)
    (if (Audio|Components|Audio|IsPlaying (Variables|Default|GetTimelineMove))
      (CallFunction|StopMoveTimeline))
    (else
      (|CallParentFunction Action Damage))))

(fn ConstructionScript
  (|CallParentFunction)
  (CallFunction|SetupHealthBar))

(fn SetupHealthBar
  (bind _returnvalue (Rendering|Material|CreateDynamicMaterialInstance (Variables|Default|GetHealthBar) 0 (.Material (Utilities|Struct|BreakMaterialSpriteElement (Utilities|Array|Get(acopy) (Variables|/Script/Engine.MaterialBillboardComponent|GetElements (Variables|Default|GetHealthBar))))) "None" :!class /Script/Engine.PrimitiveComponent))
  (bind _output_get (Variables|Default|SetHealthBarMaterial _returnvalue))
  (Rendering|Material|SetScalarParameterValue _output_get "PercentFill" (/ (Variables|Default|GetCurrentHealth) (Variables|Default|GetMaxHealth)) :!class /Script/Engine.MaterialInstanceDynamic)
  (return))

(fn ModifyHealthBar
  (params (HealthChange :type Float%20%28single-precision%29))
  (bind _currenthealth (Variables|Default|GetCurrentHealth))
  (bind _maxhealth (Variables|Default|GetMaxHealth))
  (bind _returnvalue (/ _currenthealth _maxhealth))
  (bind _returnvalue_2 (Math|Float|Max(Float) _returnvalue 0.0))
  (Rendering|Material|GetScalarParameterValue (Variables|Default|GetHealthBarMaterial) "PercentFill" :!class /Script/Engine.MaterialInstanceDynamic)
  (Rendering|Material|SetScalarParameterValue (Variables|Default|GetHealthBarMaterial) "PercentFill" (Math|Float|Min(Float) 1.0 _returnvalue_2) :!class /Script/Engine.MaterialInstanceDynamic)
  (return (== _returnvalue_2 0.0)))