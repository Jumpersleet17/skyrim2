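; BP_Unit_Player is the player unit Blueprint in the Advanced Turn Based Tile Toolkit, inheriting its behavior and CurrentAP variable from a parent class.
; Its only active event logic is a debug binding on the P key that prints CurrentAP.
; BeginPlay, overlap and Tick are disabled placeholder nodes, and the construction script only calls the parent.
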(event EventBeginPlay
  (|CallParentFunction) ; This node is disabled and will not be called.\nDrag off pins to build functionality.
)

(event Collision|EventActorBeginOverlap
  (params (OtherActor :type Actor%20Object%20Reference))
  (|CallParentFunction OtherActor) ; This node is disabled and will not be called.\nDrag off pins to build functionality.
)

(event EventTick
  (params (DeltaSeconds :type Float%20%28single-precision%29))
  (|CallParentFunction DeltaSeconds) ; This node is disabled and will not be called.\nDrag off pins to build functionality.
)

(event Input|KeyboardEvents|RightShift
  (params (Key :type Key%20Structure :default "None")))

(event Input|KeyboardEvents|P
  (params (Key :type Key%20Structure :default "None"))
  (:Pressed
    (Development|PrintString (Utilities|String|ToString(Integer) (Variables|Default|GetCurrentAP)))))

(fn ConstructionScript
  (|CallParentFunction))