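; Scene component from the turn-based tile toolkit that snaps itself and its owning actor to the grid of BP_GridManager.
; An external construction event moves the anchor to the tile closest to the owner, unless custom-grid snapping is ignored, and stores that tile's GridIndex.
; PlaceActorAtAnchor snaps the anchor's own location to a tile plus AnchorOffset, moves the owner there, then zeroes the anchor's relative location.
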(event Custom|ExternalConstuctionScript
  (bind _returnvalue (Actor|GetActorOfClass "/Game/AdvancedTurnBasedTileToolkit/Core/Grid/BP_GridManager.BP_GridManager_C"))
  (Utilities|IsValid _returnvalue
    (:Is%20Valid
      (if (Variables|Default|GetbIgnoreSnapToCustomGrid)
        (Development|PrintString "ignore custom grid")
        (else
          (bind _snaplocation (Default|FindClosestTiletoSnaptoTrace _returnvalue (Transformation|GetActorLocation (Components|GetOwner))))
          (Transformation|SetWorldLocation self _snaplocation false false)))
      (Variables|Default|SetGridIndex (.Index (Default|ConvertLocationtoIndex3D _returnvalue _snaplocation))))))

(fn PlaceActoratAnchor
  (bind _returnvalue (Actor|GetActorOfClass "/Game/AdvancedTurnBasedTileToolkit/Core/Grid/BP_GridManager.BP_GridManager_C"))
  (bind _snaplocation (Default|FindClosestTiletoSnaptoTrace _returnvalue (Transformation|GetWorldLocation)))
  (Transformation|SetWorldLocation (+ _snaplocation (Variables|Default|GetAnchorOffset)) false false)
  (Transformation|SetActorLocation (Components|GetOwner) (Transformation|GetWorldLocation) false false)
  (Transformation|SetRelativeLocation "0, 0, 0" false false)
  (return))