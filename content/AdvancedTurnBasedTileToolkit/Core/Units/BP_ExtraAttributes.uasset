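; Unit component for the turn-based tile toolkit that tracks class, level, XP and D&D-style spell slots.
; BeginPlay calls Rest, which dispatches by class; only Wizard is implemented, setting slots per level 1–20 and adding spells to the owner's BP_AbilitySystem without duplicates.
; CheckSpellSlots tests availability, while SubtractSlot spends one, rebuilds the Slots array and refreshes the HUD ability box.
; XPGain recursively handles level-ups but does not refresh slots.
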(event EventBeginPlay
  (CallFunction|Rest))

(fn XPGain
  (params (XPGained :type Float%20%28single-precision%29))
  (bind _output_get (Variables|Default|SetCurrentXP (+ XPGained (Variables|Default|GetCurrentXP))))
  (if (>= _output_get (Variables|Default|GetLvlUpXp))
    (Variables|Default|SetLevel (+ (Variables|Default|GetLevel) 1))
    (Variables|Default|SetCurrentXP (- (Variables|Default|GetCurrentXP) (Variables|Default|GetLvlUpXp)))
    (CallFunction|XPGain 0.0)
    (else
      (return))))

(fn Wizard
  (bind _spells (Variables|Default|GetSpells))
  (bind _spells_2 (Variables|Default|GetSpells))
  (bind _spells_3 (Variables|Default|GetSpells))
  (bind _spells_4 (Variables|Default|GetSpells))
  (bind _spells_5 (Variables|Default|GetSpells))
  (bind _spells_6 (Variables|Default|GetSpells))
  (bind _spells_7 (Variables|Default|GetSpells))
  (bind _spells_8 (Variables|Default|GetSpells))
  (bind _spells_9 (Variables|Default|GetSpells))
  (CallFunction|ClearSlots)
  (switch int (Variables|Default|GetLevel)
    (:1
      (Variables|Default|Set1stLevel 2)
      (CallFunction|AddAbility (Utilities|Array|Get(acopy) _spells) :!label _label)
      (CallFunction|AddAbility (Utilities|Array|Get(acopy) _spells 1))
      (CallFunction|AddAbility (Utilities|Array|Get(acopy) _spells 2)))
    (:2
      (Variables|Default|Set1stLevel 3)
      (goto _label))
    (:3
      (Variables|Default|Set1stLevel 4)
      (Variables|Default|Set2ndLevel 2)
      (CallFunction|AddAbility (Utilities|Array|Get(acopy) _spells_2) :!label _label_2)
      (CallFunction|AddAbility (Utilities|Array|Get(acopy) _spells_2 1))
      (CallFunction|AddAbility (Utilities|Array|Get(acopy) _spells_2 2)))
    (:4
      (Variables|Default|Set1stLevel 4)
      (Variables|Default|Set2ndLevel 3)
      (goto _label_2))
    (:5
      (Variables|Default|Set1stLevel 4)
      (Variables|Default|Set2ndLevel 3)
      (Variables|Default|Set3rdLevel 2)
      (CallFunction|AddAbility (Utilities|Array|Get(acopy) _spells_3) :!label _label_3)
      (CallFunction|AddAbility (Utilities|Array|Get(acopy) _spells_3 1))
      (CallFunction|AddAbility (Utilities|Array|Get(acopy) _spells_3 2)))
    (:6
      (Variables|Default|Set1stLevel 4)
      (Variables|Default|Set2ndLevel 3)
      (Variables|Default|Set3rdLevel 3)
      (goto _label_3))
    (:7
      (Variables|Default|Set1stLevel 4)
      (Variables|Default|Set2ndLevel 3)
      (Variables|Default|Set3rdLevel 3)
      (Variables|Default|Set4thLevel 1)
      (CallFunction|AddAbility (Utilities|Array|Get(acopy) _spells_4) :!label _label_4)
      (CallFunction|AddAbility (Utilities|Array|Get(acopy) _spells_4 1))
      (CallFunction|AddAbility (Utilities|Array|Get(acopy) _spells_4 2)))
    (:8
      (Variables|Default|Set1stLevel 4)
      (Variables|Default|Set2ndLevel 3)
      (Variables|Default|Set3rdLevel 3)
      (Variables|Default|Set4thLevel 2)
      (goto _label_4))
    (:9
      (Variables|Default|Set1stLevel 4)
      (Variables|Default|Set2ndLevel 3)
      (Variables|Default|Set3rdLevel 3)
      (Variables|Default|Set4thLevel 3)
      (Variables|Default|Set5thLevel 1)
      (CallFunction|AddAbility (Utilities|Array|Get(acopy) _spells_5) :!label _label_5)
      (CallFunction|AddAbility (Utilities|Array|Get(acopy) _spells_5 1))
      (CallFunction|AddAbility (Utilities|Array|Get(acopy) _spells_5 2)))
    (:10
      (Variables|Default|Set1stLevel 4)
      (Variables|Default|Set2ndLevel 3)
      (Variables|Default|Set3rdLevel 3)
      (Variables|Default|Set4thLevel 3)
      (Variables|Default|Set5thLevel 2)
      (goto _label_5))
    (:11
      (Variables|Default|Set1stLevel 4)
      (Variables|Default|Set2ndLevel 3)
      (Variables|Default|Set3rdLevel 3)
      (Variables|Default|Set4thLevel 3)
      (Variables|Default|Set5thLevel 2)
      (Variables|Default|Set6thLevel 1)
      (CallFunction|AddAbility (Utilities|Array|Get(acopy) _spells_6) :!label _label_6)
      (CallFunction|AddAbility (Utilities|Array|Get(acopy) _spells_6 1))
      (CallFunction|AddAbility (Utilities|Array|Get(acopy) _spells_6 2)))
    (:12
      (Variables|Default|Set1stLevel 4)
      (Variables|Default|Set2ndLevel 3)
      (Variables|Default|Set3rdLevel 3)
      (Variables|Default|Set4thLevel 3)
      (Variables|Default|Set5thLevel 2)
      (Variables|Default|Set6thLevel 1)
      (goto _label_6))
    (:13
      (Variables|Default|Set1stLevel 4)
      (Variables|Default|Set2ndLevel 3)
      (Variables|Default|Set3rdLevel 3)
      (Variables|Default|Set4thLevel 3)
      (Variables|Default|Set5thLevel 2)
      (Variables|Default|Set6thLevel 1)
      (Variables|Default|Set7thLevel 1)
      (CallFunction|AddAbility (Utilities|Array|Get(acopy) _spells_8) :!label _label_7)
      (CallFunction|AddAbility (Utilities|Array|Get(acopy) _spells_8 1))
      (CallFunction|AddAbility (Utilities|Array|Get(acopy) _spells_8 2)))
    (:14
      (Variables|Default|Set1stLevel 4)
      (Variables|Default|Set2ndLevel 3)
      (Variables|Default|Set3rdLevel 3)
      (Variables|Default|Set4thLevel 3)
      (Variables|Default|Set5thLevel 2)
      (Variables|Default|Set6thLevel 1)
      (Variables|Default|Set7thLevel 1)
      (goto _label_7))
    (:15
      (Variables|Default|Set1stLevel 4)
      (Variables|Default|Set2ndLevel 3)
      (Variables|Default|Set3rdLevel 3)
      (Variables|Default|Set4thLevel 3)
      (Variables|Default|Set5thLevel 2)
      (Variables|Default|Set6thLevel 1)
      (Variables|Default|Set7thLevel 1)
      (Variables|Default|Set8thLevel 1)
      (CallFunction|AddAbility (Utilities|Array|Get(acopy) _spells_9) :!label _label_8)
      (CallFunction|AddAbility (Utilities|Array|Get(acopy) _spells_9 1))
      (CallFunction|AddAbility (Utilities|Array|Get(acopy) _spells_9 2)))
    (:16
      (Variables|Default|Set1stLevel 4)
      (Variables|Default|Set2ndLevel 3)
      (Variables|Default|Set3rdLevel 3)
      (Variables|Default|Set4thLevel 3)
      (Variables|Default|Set5thLevel 2)
      (Variables|Default|Set6thLevel 1)
      (Variables|Default|Set7thLevel 1)
      (Variables|Default|Set8thLevel 1)
      (goto _label_8))
    (:17
      (Variables|Default|Set1stLevel 4)
      (Variables|Default|Set2ndLevel 3)
      (Variables|Default|Set3rdLevel 3)
      (Variables|Default|Set4thLevel 3)
      (Variables|Default|Set5thLevel 2)
      (Variables|Default|Set6thLevel 1)
      (Variables|Default|Set7thLevel 1)
      (Variables|Default|Set8thLevel 1)
      (Variables|Default|Set9thLevel 1)
      (CallFunction|AddAbility (Utilities|Array|Get(acopy) _spells_7) :!label _label_9)
      (CallFunction|AddAbility (Utilities|Array|Get(acopy) _spells_7 1))
      (CallFunction|AddAbility (Utilities|Array|Get(acopy) _spells_7 2)))
    (:18
      (Variables|Default|Set1stLevel 4)
      (Variables|Default|Set2ndLevel 3)
      (Variables|Default|Set3rdLevel 3)
      (Variables|Default|Set4thLevel 3)
      (Variables|Default|Set5thLevel 3)
      (Variables|Default|Set6thLevel 1)
      (Variables|Default|Set7thLevel 1)
      (Variables|Default|Set8thLevel 1)
      (Variables|Default|Set9thLevel 1)
      (goto _label_9))
    (:19
      (Variables|Default|Set1stLevel 4)
      (Variables|Default|Set2ndLevel 3)
      (Variables|Default|Set3rdLevel 3)
      (Variables|Default|Set4thLevel 3)
      (Variables|Default|Set5thLevel 3)
      (Variables|Default|Set6thLevel 2)
      (Variables|Default|Set7thLevel 1)
      (Variables|Default|Set8thLevel 1)
      (Variables|Default|Set9thLevel 1)
      (goto _label_9))
    (:20
      (Variables|Default|Set1stLevel 4)
      (Variables|Default|Set2ndLevel 3)
      (Variables|Default|Set3rdLevel 3)
      (Variables|Default|Set4thLevel 3)
      (Variables|Default|Set5thLevel 3)
      (Variables|Default|Set6thLevel 2)
      (Variables|Default|Set7thLevel 2)
      (Variables|Default|Set8thLevel 1)
      (Variables|Default|Set9thLevel 1)
      (goto _label_9)))
  (CallFunction|SetSlots))

(fn Rest
  (switch string (Variables|Default|GetMyClass)
    (:Wizard
      (CallFunction|Wizard))
    (:Fighter
      (CallFunction|Fighter))
    (:Rouge
      (CallFunction|Rogue))
    (:Ranger
      (CallFunction|Ranger))))

(fn AddAbility
  (params (AbilityToCheck :type BP%20Ability%20Class%20Reference))
  (bind _returnvalue (Components|GetOwner))
  (bind _returnvalue_2 (Actor|GetComponentbyClass _returnvalue "/Game/AdvancedTurnBasedTileToolkit/Core/Units/BP_AbilitySystem.BP_AbilitySystem_C"))
  (bind _bhasability (Default|CheckifHasAbility _returnvalue_2 AbilityToCheck))
  (if (not _bhasability)
    (Utilities|Array|Add (Variables|/Game/AdvancedTurnBasedTileToolkit/Core/Units/BP_AbilitySystem.BP_AbilitySystem_C|GetAbilities _returnvalue_2) AbilityToCheck)))

(fn Ranger)

(fn Fighter)

(fn Rogue)

(fn CheckSpellSlots
  (params (SpellSlot :type Integer))
  (switch int SpellSlot
    (:1
      (if (> (Variables|Default|Get1stLevel) 0)
        (return true)
        (else
          (return false))))
    (:2
      (if (> (Variables|Default|Get2ndLevel) 0)
        (return true)
        (else
          (return false))))
    (:3
      (if (> (Variables|Default|Get3rdLevel) 0)
        (return true)
        (else
          (return false))))
    (:4
      (if (> (Variables|Default|Get4thLevel) 0)
        (return true)
        (else
          (return false))))
    (:5
      (if (> (Variables|Default|Get5thLevel) 0)
        (return true)
        (else
          (return false))))
    (:6
      (if (> (Variables|Default|Get6thLevel) 0)
        (return true)
        (else
          (return false))))
    (:7
      (if (> (Variables|Default|Get7thLevel) 0)
        (return true)
        (else
          (return false))))
    (:8
      (if (> (Variables|Default|Get8thLevel) 0)
        (return true)
        (else
          (return false))))
    (:9
      (if (> (Variables|Default|Get9thLevel) 0)
        (return true)
        (else
          (return false))))))

(fn SubtractSlot
  (params (SpellSlot :type Integer))
  (switch int SpellSlot
    (:1
      (Variables|Default|Set1stLevel (- (Variables|Default|Get1stLevel) 1)))
    (:2
      (Variables|Default|Set2ndLevel (- (Variables|Default|Get2ndLevel) 1)))
    (:3
      (Variables|Default|Set3rdLevel (- (Variables|Default|Get3rdLevel) 1)))
    (:4
      (Variables|Default|Set4thLevel (- (Variables|Default|Get4thLevel) 1)))
    (:5
      (Variables|Default|Set5thLevel (- (Variables|Default|Get5thLevel) 1)))
    (:6
      (Variables|Default|Set6thLevel (- (Variables|Default|Get6thLevel) 1)))
    (:7
      (Variables|Default|Set7thLevel (- (Variables|Default|Get7thLevel) 1)))
    (:8
      (Variables|Default|Set8thLevel (- (Variables|Default|Get8thLevel) 1)))
    (:9
      (Variables|Default|Set9thLevel (- (Variables|Default|Get9thLevel) 1))))
  (CallFunction|ClearSlots)
  (CallFunction|SetSlots)
  (bind _returnvalue (Actor|GetActorOfClass "/Game/AdvancedTurnBasedTileToolkit/Core/UI/BP_HUD_ATBTT.BP_HUD_ATBTT_C"))
  (Default|SetText (Variables|/Game/AdvancedTurnBasedTileToolkit/Core/UI/WBP_ATBTT.WBP_ATBTT_C|GetWBP_AbilityBox (Variables|/Game/AdvancedTurnBasedTileToolkit/Core/UI/BP_HUD_ATBTT.BP_HUD_ATBTT_C|GetWbpAtbttRef _returnvalue))))

(fn SetSlots
  (bind _slots (Variables|Default|GetSlots))
  (Utilities|Array|Add _slots (Variables|Default|Get1stLevel))
  (Utilities|Array|Add _slots (Variables|Default|Get2ndLevel))
  (Utilities|Array|Add _slots (Variables|Default|Get3rdLevel))
  (Utilities|Array|Add _slots (Variables|Default|Get4thLevel))
  (Utilities|Array|Add _slots (Variables|Default|Get5thLevel))
  (Utilities|Array|Add _slots (Variables|Default|Get6thLevel))
  (Utilities|Array|Add _slots (Variables|Default|Get7thLevel))
  (Utilities|Array|Add _slots (Variables|Default|Get8thLevel))
  (Utilities|Array|Add _slots (Variables|Default|Get9thLevel))
  (Variables|Default|SetSlotsReady true)
  (return))

(fn ClearSlots
  (Utilities|Array|Clear (Variables|Default|GetSlots))
  (Variables|Default|SetSlotsReady false))