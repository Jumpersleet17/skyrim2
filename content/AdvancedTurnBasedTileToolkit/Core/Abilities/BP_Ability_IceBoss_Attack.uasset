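; Ice boss attack ability for the turn-based tile toolkit that adds an ice hit particle effect to its parent ability's attack.
; On AttackHit it looks up the unit at the target index in the grid manager's GridUnits and, if valid, attaches the emitter to that unit's scene component.
; It then calls the parent AttackHit, which handles the rest of the hit.
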(event EventBeginPlay
  (|CallParentFunction) ; This node is disabled and will not be called.\nDrag off pins to build functionality.
)

(event Collision|EventActorBeginOverlap
  (params (OtherActor :type Actor%20Object%20Reference)))

(event EventTick
  (params (DeltaSeconds :type Float%20%28single-precision%29)))

(event EventAttackHit
  (bind _gridmanagerref (Variables|Default|GetGridManagerRef))
  (bind _targetindex (Variables|Default|GetTargetIndex))
  (bind _gridunits (Variables|/Game/AdvancedTurnBasedTileToolkit/Core/Grid/BP_GridManager.BP_GridManager_C|GetGridUnits _gridmanagerref))
  (bind _value (Utilities|Map|Find _gridunits _targetindex))
  (if (Utilities|IsValid _value)
    (Effects|SpawnEmitterAttached "/Game/AdvancedMagicFX12/particles/P_ky_hit_ice.P_ky_hit_ice" (Variables|/Game/AdvancedTurnBasedTileToolkit/Core/Grid/BP_GridActor.BP_GridActor_C|GetSceneComponent _value) "None"))
  (|CallParentFunction))

(fn ConstructionScript
  (|CallParentFunction))