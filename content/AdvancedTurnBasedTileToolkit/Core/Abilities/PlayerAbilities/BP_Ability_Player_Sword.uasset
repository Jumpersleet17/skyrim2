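; Player sword slash ability for the turn-based tile toolkit, used to strike an enemy.
; ExecuteAbility looks up the unit at the target index in the grid manager's GridUnits map and attaches a slash hit particle to it.
; It then defers to the parent ability's ExecuteAbility and returns that result.
; GetDescription supplies the ability's description text.
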(event EventBeginPlay
  (|CallParentFunction) ; This node is disabled and will not be called.\nDrag off pins to build functionality.
)

(event Collision|EventActorBeginOverlap
  (params (OtherActor :type Actor%20Object%20Reference)))

(event EventTick
  (params (DeltaSeconds :type Float%20%28single-precision%29)))

(fn ConstructionScript
  (|CallParentFunction))

(fn ExecuteAbility
  (params (TargetIndex :type Integer) (D20Die :type D20%20Dice%20BP%20Object%20Reference))
  (Effects|SpawnEmitterAttached "/Game/AdvancedMagicFX13/Particles/P_ky_hit_slash.P_ky_hit_slash" (Variables|/Game/AdvancedTurnBasedTileToolkit/Core/Grid/BP_GridActor.BP_GridActor_C|GetSceneComponent (.Value (Utilities|Map|Find (Variables|/Game/AdvancedTurnBasedTileToolkit/Core/Grid/BP_GridManager.BP_GridManager_C|GetGridUnits (Variables|Default|GetGridManagerRef)) TargetIndex))) "None")
  (bind _bsuccess (|CallParentFunction TargetIndex 0))
  (return _bsuccess))

(fn GetDescription
  (return "Sword Slash: 
Slash an enemy with your sword."))