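; Status effect Blueprint for the turn-based tile toolkit that marks a unit as woke and disables itself when its turn-start event runs.
; Its activation animation pans the player pawn to the owning unit, reveals an indicator, plays a random spot sound, waits, then ends the action through the game state.
; The wait re-rolls the random sound index, so its duration can differ from the sound played.
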(event EventRunonTurnStart
  (CallFunction|Disable))

(event EventAnimateActivation
  (bind _spotsounds (Variables|Default|GetSpotSounds))
  (bind _owningunit (Variables|Default|GetOwningUnit))
  (bind _returnvalue (Utilities|Array|Length _spotsounds))
  (bind _returnvalue_2 (Transformation|GetActorLocation _owningunit))
  (bind _returnvalue_3 (- _returnvalue 1))
  (bind _returnvalue_4 (Math|Random|RandomInteger _returnvalue_3))
  (bind _output (Utilities|Array|Get(acopy) _spotsounds _returnvalue_4))
  (Class|BPICameraControls|PantoLocation(Message) (Game|Player|GetPlayerPawn 0) _returnvalue_2)
  (Utilities|FlowControl|Delay 0.6)
  (Rendering|SetVisibility (Variables|Default|GetEffectIndicator) true false)
  (Audio|PlaySoundatLocation _output _returnvalue_2 "0, 0, 0" 1.0 1.0 0.0 0 0 0)
  (Utilities|FlowControl|Delay (Variables|/Script/Engine.SoundBase|GetDuration _output))
  (Class|BPIAction|EndAction(Message) (Game|GetGameState)))

(fn ConstructionScript
  (|CallParentFunction))