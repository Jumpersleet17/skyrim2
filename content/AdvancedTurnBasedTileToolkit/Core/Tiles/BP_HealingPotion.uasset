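; Healing potion grid pickup for the turn-based tile toolkit that heals a player unit on overlap when OverlapInteract is enabled.
; Overlap rolls a random negative SuccessDamage, which GetSuccess passes to TakeDamage as healing.
; GetSuccess also applies gold, arrows and any ability, refreshes the UI, then removes the potion from grid and world.
; Its popup text is disconnected; GetFailure has a popup and penalty path but is not called here.
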(event EventBeginPlay)

(event Collision|EventActorBeginOverlap
  (params (OtherActor :type Actor%20Object%20Reference))
  (Variables|Default|SetSuccessDamage (Math|Random|RandomIntegerinRange -100 -40))
  (if (Variables|Default|GetOverlapInteract)
    (bind _asbp_unit_player (Utilities|Casting|CastToBP_Unit_Player OtherActor))
    (CallFunction|GetSuccess _asbp_unit_player)))

(event EventTick
  (params (DeltaSeconds :type Float%20%28single-precision%29)))

(fn ConstructionScript)

(fn GetSuccess
  (params (Target :type BP%20Unit%20Player%20Object%20Reference))
  (bind _bp_abilitysystem (Variables|/Game/AdvancedTurnBasedTileToolkit/Units/BP_Unit_Anim_AdvTemp.BP_Unit_Anim_AdvTemp_C|GetBP_AbilitySystem Target))
  (Default|TakeDamage Target (Math|Conversions|ToFloat(Integer) (Variables|Default|GetSuccessDamage)) false)
  (bind _output_get (Variables|/Game/AdvancedTurnBasedTileToolkit/Core/Units/BP_Unit.BP_Unit_C|SetcurrentGold Target (+ (Variables|/Game/AdvancedTurnBasedTileToolkit/Core/Units/BP_Unit.BP_Unit_C|GetcurrentGold Target) (Variables|Default|GetSuccessGold))))
  (if (< _output_get 0)
    (Variables|/Game/AdvancedTurnBasedTileToolkit/Core/Units/BP_Unit.BP_Unit_C|SetcurrentGold Target 0))
  (Variables|/Game/AdvancedTurnBasedTileToolkit/Core/Units/BP_Unit.BP_Unit_C|SetArrowCount Target (+ (Variables|/Game/AdvancedTurnBasedTileToolkit/Core/Units/BP_Unit.BP_Unit_C|GetArrowCount Target) (Variables|Default|GetSuccessArrows)))
  (bind _foundwidgets (Widget|GetAllWidgetsOfClass "/Game/AdvancedTurnBasedTileToolkit/Core/UI/WBP_ATBTT.WBP_ATBTT_C" true))
  (for _array_element _foundwidgets
    (Rendering|Components|TextRender|SetText (Variables|/Game/AdvancedTurnBasedTileToolkit/Core/UI/WBP_AbilityBox.WBP_AbilityBox_C|GetGoldBox (Variables|/Game/AdvancedTurnBasedTileToolkit/Core/UI/WBP_ATBTT.WBP_ATBTT_C|GetWBP_AbilityBox _array_element)) (Utilities|Text|ToText(Integer) _output_get)))
  (if (Utilities|IsValidClass (Variables|Default|GetAbility_or_Weapon_Gained))
    (Utilities|Array|Add (Variables|/Game/AdvancedTurnBasedTileToolkit/Core/Units/BP_AbilitySystem.BP_AbilitySystem_C|GetAbilities _bp_abilitysystem) (Variables|Default|GetAbility_or_Weapon_Gained))
    (Default|UpdateRefences _bp_abilitysystem)
    (Default|UpdateAbilityBox Target))
  (Default|RemoveObjectfromGrid (Variables|Default|GetGridManagerRef) self (Variables|Default|GetGridIndex))
  (Actor|DestroyActor))

(fn GetFailure
  (params (Target :type BP%20Unit%20Player%20Object%20Reference))
  (bind _returnvalue (UserInterface|CreateWidget "/Game/AdvancedTurnBasedTileToolkit/Core/UI/PerceptionText.PerceptionText_C" (Game|GetPlayerController 0)))
  (Rendering|Components|TextRender|SetText (Variables|/Game/AdvancedTurnBasedTileToolkit/Core/UI/PerceptionText.PerceptionText_C|GetActualText _returnvalue) (Utilities|Text|ToText(String) (Variables|Default|GetFailure%20Text)))
  (UserInterface|Viewport|AddtoViewport _returnvalue 0)
  (Default|TakeDamage Target (Math|Conversions|ToFloat(Integer) (Variables|Default|GetFailureDamage)) false)
  (bind _output_get (Variables|/Game/AdvancedTurnBasedTileToolkit/Core/Units/BP_Unit.BP_Unit_C|SetcurrentGold Target (+ (Variables|/Game/AdvancedTurnBasedTileToolkit/Core/Units/BP_Unit.BP_Unit_C|GetcurrentGold Target) (Variables|Default|GetFailureGold))))
  (if (< _output_get 0)
    (Variables|/Game/AdvancedTurnBasedTileToolkit/Core/Units/BP_Unit.BP_Unit_C|SetcurrentGold Target 0))
  (Variables|/Game/AdvancedTurnBasedTileToolkit/Core/Units/BP_Unit.BP_Unit_C|SetArrowCount Target (+ (Variables|/Game/AdvancedTurnBasedTileToolkit/Core/Units/BP_Unit.BP_Unit_C|GetArrowCount Target) (Variables|Default|GetFailureArrows)))
  (bind _foundwidgets (Widget|GetAllWidgetsOfClass "/Game/AdvancedTurnBasedTileToolkit/Core/UI/WBP_ATBTT.WBP_ATBTT_C" true))
  (for _array_element _foundwidgets
    (Rendering|Components|TextRender|SetText (Variables|/Game/AdvancedTurnBasedTileToolkit/Core/UI/WBP_AbilityBox.WBP_AbilityBox_C|GetGoldBox (Variables|/Game/AdvancedTurnBasedTileToolkit/Core/UI/WBP_ATBTT.WBP_ATBTT_C|GetWBP_AbilityBox _array_element)) (Utilities|Text|ToText(Integer) _output_get))
    (Default|RemoveObjectfromGrid (Variables|Default|GetGridManagerRef) self (Variables|Default|GetGridIndex))
    (Actor|DestroyActor)))