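; BP_Action_Teleport is a turn-based action in the Advanced Turn Based Tile Toolkit that visually teleports a puppet to a target location.
; When played, it hides the puppet, waits, moves it to the target without sweeping, and waits again.
; It then spawns an explosion effect with a fireblast sound there, reveals the puppet and ends the action.
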(event EventPlayAction
  (bind _targetlocation (Variables|Default|GetTargetLocation))
  (Rendering|SetActorHiddenInGame (Variables|Default|GetPuppet) true)
  (Utilities|FlowControl|Delay 1.0)
  (Transformation|SetActorLocation (Variables|Default|GetPuppet) (Variables|Default|GetTargetLocation) false false)
  (Utilities|FlowControl|Delay 1.0)
  (Effects|SpawnEmitteratLocation "/Game/AdvancedTurnBasedTileToolkit/Maps/Advanced/Abilities/PS_Explosion.PS_Explosion" _targetlocation "0, 0, 0" "2.000000,2.000000,2.000000")
  (Audio|PlaySoundatLocation "/Game/AdvancedTurnBasedTileToolkit/Maps/Advanced/Abilities/A_Fireblast.A_Fireblast" _targetlocation "0, 0, 0" 1.0 1.0 0.0 0 0 0)
  (Rendering|SetActorHiddenInGame (Variables|Default|GetPuppet) false)
  (CallFunction|EndAction))

(fn ConstructionScript
  (|CallParentFunction))