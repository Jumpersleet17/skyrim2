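; Debug unit Blueprint for the teleport action in the Advanced Turn Based Tile Toolkit, apparently a variant of an animated unit.
; QueueOrExtendMoveAction clears SkipNextMoveAction when it is set and returns on both branches, so this function never queues or extends a move action.
; The event graph holds only disabled default events, and the construction script just calls its parent.
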(event EventBeginPlay
  (|CallParentFunction) ; This node is disabled and will not be called.\nDrag off pins to build functionality.
)

(event Collision|EventActorBeginOverlap
  (params (OtherActor :type Actor%20Object%20Reference))
  (|CallParentFunction OtherActor) ; This node is disabled and will not be called.\nDrag off pins to build functionality.
)

(event EventTick
  (params (DeltaSeconds :type Float%20%28single-precision%29))
  (|CallParentFunction DeltaSeconds) ; This node is disabled and will not be called.\nDrag off pins to build functionality.
)

(fn ConstructionScript
  (|CallParentFunction))

(fn QueueorExtendMoveAction
  (params (ActionManager :type BP%20Action%20Manager%20Object%20Reference) (MoveSource :type Vector :default "0, 0, 0") (MoveTarget :type Vector :default "0, 0, 0") (bStartOfMove :type Boolean) (bEndOfMove :type Boolean))
  (if (Variables|Default|GetSkipNextMoveAction)
    (Variables|Default|SetSkipNextMoveAction false)
    (return)
    (else
      (return))))