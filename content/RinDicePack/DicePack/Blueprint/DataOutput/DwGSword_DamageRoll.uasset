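; Damage roll display, apparently for a GSword weapon, that shows the combined result of two D6 numbered dice.
; Every Tick, it casts both referenced dice to D6_Num_Dice_BP, adds their DiceResultData and writes the sum to the DataValue text.
; An unconnected loop that would spawn scaled-up dice at the player's location and display their results never runs.
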(event EventTick
  (params (DeltaSeconds :type Float%20%28single-precision%29))
  ;[1 1 1] Read selected from level D6_NumDice Data
  (bind _asd6_num_dice_bp (Utilities|Casting|CastToD6_Num_Dice_BP (Variables|Default|GetDiceToCheck)))
  (bind _asd6_num_dice_bp_2 (Utilities|Casting|CastToD6_Num_Dice_BP (Variables|Default|GetDiceToCheck_2)))
  (Rendering|Components|TextRender|SetText (Variables|Default|GetDataValue) (Utilities|Text|ToText(String) (Utilities|String|ToString(Integer) (+ (Variables|/Game/RinDicePack/D6_Num_Dice_BP.D6_Num_Dice_BP_C|GetDiceResultData _asd6_num_dice_bp) (Variables|/Game/RinDicePack/D6_Num_Dice_BP.D6_Num_Dice_BP_C|GetDiceResultData _asd6_num_dice_bp_2))))))

(fn ConstructionScript)