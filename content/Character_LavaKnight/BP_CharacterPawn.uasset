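; BP_CharacterPawn is a player-controlled pawn in the Lava Knight character folder, handling basic look and movement input.
; LookUp and Turn axes feed controller pitch and yaw directly.
; MoveForward and MoveRight rotate unit X and Y vectors by the control rotation's yaw only, so movement follows the view heading and stays horizontal regardless of pitch.
; The construction script is empty.
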(event Input|AxisEvents|InputAxisLookUp
  (params (AxisValue :type Float%20%28single-precision%29))
  (Pawn|Input|AddControllerPitchInput AxisValue))

(event Input|AxisEvents|InputAxisTurn
  (params (AxisValue :type Float%20%28single-precision%29))
  (Pawn|Input|AddControllerYawInput AxisValue))

(event Input|AxisEvents|InputAxisMoveForward
  (params (AxisValue :type Float%20%28single-precision%29))
  (Pawn|Input|AddMovementInput (Math|Vector|RotateVector "1.000000, 0, 0" (Math|Rotator|MakeRotator 0.0 0.0 (.Yaw (Math|Rotator|BreakRotator (Pawn|GetControlRotation (Pawn|GetController) :!class /Script/Engine.Controller))))) AxisValue false))

(event Input|AxisEvents|InputAxisMoveRight
  (params (AxisValue :type Float%20%28single-precision%29))
  (Pawn|Input|AddMovementInput (Math|Vector|RotateVector "0,1.000000, 0" (Math|Rotator|MakeRotator 0.0 0.0 (.Yaw (Math|Rotator|BreakRotator (Pawn|GetControlRotation (Pawn|GetController) :!class /Script/Engine.Controller))))) AxisValue false))

(fn ConstructionScript)